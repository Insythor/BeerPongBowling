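; BP_Twomp is a Thwomp-style hazard that drops when the physics ball passes through its trigger.
; A timeline lerps the Thwomp's relative location from StartLoc to the EndLoc component, then resets its playhead after finishing.
; Any overlap with the Death volume reloads RollingBPExampleMap, without filtering by actor.
; With BeginOnPlay set, separate up or down timelines, chosen by MoveUp, also move it automatically as background motion.
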(event OnComponentBeginOverlap(Trigger)
  (params (OverlappedComponent :type Primitive%20Component%20Object%20Reference) (OtherActor :type Actor%20Object%20Reference) (OtherComp :type Primitive%20Component%20Object%20Reference) (OtherBodyIndex :type Integer) (bFromSweep :type Boolean) (SweepResult :type Hit%20Result%20Structure%20%28by%20ref%29))
  ;[0 0 0] When player passes through the Collision Box, Lower the THWOMP
  (Utilities|Casting|CastToPhysicsBallBP OtherActor)
  (bind _movement (Timeline|Thwomp%20Movement Play)
    (:Update
      (Transformation|SetRelativeLocation (Variables|Default|GetThwomp) (Math|Vector|Lerp(Vector) (Math|Conversions|ToVector(Float) (Variables|Default|GetStartLoc)) (Variables|/Script/Engine.SceneComponent|GetRelativeLocation (Variables|Default|GetEndLoc)) _movement) false false))
    (:Finished
      (Utilities|FlowControl|Delay 0.0001)
      (Timeline|Thwomp%20Movement SetNewTime))))

(event OnComponentBeginOverlap(Death)
  (params (OverlappedComponent :type Primitive%20Component%20Object%20Reference) (OtherActor :type Actor%20Object%20Reference) (OtherComp :type Primitive%20Component%20Object%20Reference) (OtherBodyIndex :type Integer) (bFromSweep :type Boolean) (SweepResult :type Hit%20Result%20Structure%20%28by%20ref%29))
  ;[0 0 0] Restarts level if Hit by Thwomp
  (Game|OpenLevel(byName) "RollingBPExampleMap"))

(event EventBeginPlay
  ;[0 0 0] Automatic movement either Up or Down, just for Background stuff
  (if (Variables|Default|GetBegin%20On%20Play)
    (if (Variables|Default|GetMove%20Up)
      (bind _movement (Timeline|Automatic%20Movement%20Up Play)
        (:Update
          (Transformation|SetRelativeLocation (Variables|Default|GetThwomp) (Math|Vector|Lerp(Vector) (Math|Conversions|ToVector(Float) (Variables|Default|GetStartLoc)) (Variables|/Script/Engine.SceneComponent|GetRelativeLocation (Variables|Default|GetEndLoc)) _movement) false false)))
      (else
        (bind _movement_2 (Timeline|Automatic%20Movement%20Down Play)
          (:Update
            (Transformation|SetRelativeLocation (Variables|Default|GetThwomp) (Math|Vector|Lerp(Vector) (Math|Conversions|ToVector(Float) (Variables|Default|GetStartLoc)) (Variables|/Script/Engine.SceneComponent|GetRelativeLocation (Variables|Default|GetEndLoc)) _movement_2) false false)))))))

(fn ConstructionScript)