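; Trigger-activated bridge that moves a platform while the physics ball overlaps its trigger.
; On overlap, it calls a play-sound node at the platform, waits briefly, then plays the ForwardMovement timeline.
; The timeline lerps the platform's relative location from StartLoc to the EndLocation component's relative position.
; When the ball leaves, the timeline reverses immediately, returning the platform toward its start.
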(event OnComponentEndOverlap(Trigger)
  (params (OverlappedComponent :type Primitive%20Component%20Object%20Reference) (OtherActor :type Actor%20Object%20Reference) (OtherComp :type Primitive%20Component%20Object%20Reference) (OtherBodyIndex :type Integer))
  ;[1 1 1] The following only occurs if the ball stops touching the trigger
  (Utilities|Casting|CastToPhysicsBallBP OtherActor)
  (bind _movement_forward (Timeline|ForwardMovement Reverse)
    (:Update
      (Transformation|SetRelativeLocation (Variables|Default|GetActivatedPlatform) (Math|Vector|Lerp(Vector) (Variables|Default|GetStartLoc) (Variables|/Script/Engine.SceneComponent|GetRelativeLocation (Variables|Default|GetEndLocation)) _movement_forward) false false))))

(event OnComponentBeginOverlap(Trigger)
  (params (OverlappedComponent :type Primitive%20Component%20Object%20Reference) (OtherActor :type Actor%20Object%20Reference) (OtherComp :type Primitive%20Component%20Object%20Reference) (OtherBodyIndex :type Integer) (bFromSweep :type Boolean) (SweepResult :type Hit%20Result%20Structure%20%28by%20ref%29))
  ;[1 1 1] The following only occurs if the ball touches the trigger
  (Utilities|Casting|CastToPhysicsBallBP OtherActor)
  ;[1 1 1] Add Sound Here
  (Audio|PlaySoundatLocation 0 (Transformation|GetWorldLocation (Variables|Default|GetActivatedPlatform)) "0, 0, 0" 1.0 1.0 0.0 0 0 0)
  (Utilities|FlowControl|Delay 0.5)
  (bind _movement_forward (Timeline|ForwardMovement Play)
    (:Update
      (Transformation|SetRelativeLocation (Variables|Default|GetActivatedPlatform) (Math|Vector|Lerp(Vector) (Variables|Default|GetStartLoc) (Variables|/Script/Engine.SceneComponent|GetRelativeLocation (Variables|Default|GetEndLocation)) _movement_forward) false false))))

(event EventBeginPlay)

(event Collision|EventActorBeginOverlap
  (params (OtherActor :type Actor%20Object%20Reference)))

(event EventTick
  (params (DeltaSeconds :type Float%20%28single-precision%29)))

(fn ConstructionScript)