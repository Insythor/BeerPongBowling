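; BP_BallChaser is a physics-driven ball chaser that rolls after the player pawn and opens RollingBPExampleMap when its trigger overlaps a PhysicsBallBP.
; While chasing, Tick applies acceleration-based torque separately for the world X and Y offsets, scaled by distance so the push weakens as it closes in.
; On BeginPlay it binds to BallChaser_TriggerCollision actors, whose event toggles chasing on and off through a FlipFlop.
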(event OnComponentBeginOverlap(Trigger)
  (params (OverlappedComponent :type Primitive%20Component%20Object%20Reference) (OtherActor :type Actor%20Object%20Reference) (OtherComp :type Primitive%20Component%20Object%20Reference) (OtherBodyIndex :type Integer) (bFromSweep :type Boolean) (SweepResult :type Hit%20Result%20Structure%20%28by%20ref%29))
  (Utilities|Casting|CastToPhysicsBallBP OtherActor)
  (Game|OpenLevel(byName) "RollingBPExampleMap"))

(event Custom|Chase%20Player%20ON/OFF
  ;[0 0 0] Turns the Chase Player function On/Off
  (Utilities|FlowControl|FlipFlop
    (:A
      (Variables|Default|SetChase%20Player true))
    (:B
      (Variables|Default|SetChase%20Player false))))

(event EventBeginPlay
  ;[0 0 0] Turns the Chase Player function On/Off
  (bind _outactors (Actor|GetAllActorsOfClass "/Game/Blueprints/Chasers/BallChaser_TriggerCollision.BallChaser_TriggerCollision_C"))
  (EventDispatchers|BindEventtoInitializeChase _outactors (delegate Custom|Chase%20Player%20ON/OFF)))

(event EventTick
  (params (DeltaSeconds :type Float%20%28single-precision%29))
  (bind _returnvalue (Game|Player|GetPlayerPawn 0))
  (bind _chaser (Variables|Default|GetChaser))
  (bind _zerovar (Variables|Default|GetZeroVar))
  (bind _accelchange (Variables|Default|GetAccelChange))
  (bind _zerovar_2 (Variables|Default|GetZeroVar))
  (bind _accelchange_2 (Variables|Default|GetAccelChange))
  (bind _chaser_2 (Variables|Default|GetChaser))
  (bind _returnvalue_2 (Transformation|GetWorldLocation _chaser))
  (bind _rootcomponent (Variables|/Script/Engine.Actor|GetRootComponent _returnvalue))
  (bind _returnvalue_3 (Transformation|GetWorldLocation _rootcomponent))
  (bind _returnvalue_4 (- (.y _returnvalue_3) (.y _returnvalue_2)))
  (bind _returnvalue_5 (- (.x _returnvalue_3) (.x _returnvalue_2)))
  (bind _returnvalue_6 (Math|Float|Absolute(Float) _returnvalue_4))
  (bind _returnvalue_7 (Math|Float|Absolute(Float) _returnvalue_5))
  (bind _returnvalue_8 (Math|Float|NormalizetoRange _returnvalue_6 0.0 1e+03))
  (bind _returnvalue_9 (Math|Float|NormalizetoRange _returnvalue_7 0.0 1e+03))
  (bind _returnvalue_10 (Math|Float|Lerp _zerovar _accelchange _returnvalue_8))
  (bind _returnvalue_11 (Math|Float|Lerp _zerovar_2 _accelchange_2 _returnvalue_9))
  (if (Variables|Default|GetChase%20Player)
    (Utilities|FlowControl|Sequence
      (:then_0
        (if (>= (.x _returnvalue_3) (.x _returnvalue_2))
          (Class|PrimitiveComponent|AddTorqueinRadians _chaser_2 (Math|Vector|MakeVector 0.0 _returnvalue_11 0.0) "None" true)
          (else
            (Class|PrimitiveComponent|AddTorqueinRadians _chaser_2 (Math|Vector|MakeVector 0.0 (* -1 _returnvalue_11) 0.0) "None" true))))
      (:then_1
        (if (>= (.y _returnvalue_3) (.y _returnvalue_2))
          (Class|PrimitiveComponent|AddTorqueinRadians _chaser_2 (Math|Vector|MakeVector (* -1 _returnvalue_10) 0.0 0.0) "None" true)
          (else
            (Class|PrimitiveComponent|AddTorqueinRadians _chaser_2 (Math|Vector|MakeVector _returnvalue_10 0.0 0.0) "None" true)))))))

(fn ConstructionScript)