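; Platform_Negative is a moving platform that starts travelling when play begins, with its offset driven by a timeline.
; BeginPlay stores the Platform component's world location and sets the timeline length from PlatformMovementTime.
; Each timeline update adds XMovementDistance to that stored location and applies it as the actor's relative location, without sweep.
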(event EventBeginPlay
  ;[0.07812 0.07812 0.07812] Initialized a Vector to store original playform location,
  ; to use as a reference for the movement
  (Variables|Default|SetInitial%20Platform%20Location (Transformation|GetWorldLocation (Variables|Default|GetPlatform)))
  (Components|Timeline|SetTimelineLength (Variables|Default|GetPlatformMovement_Timeline%202) (Variables|Default|GetPlatform%20Movement%20Time)) ; Sets the Duration of the Platform movement
  ;[0.09375 0.09375 0.09375] Moves the platform Positive on the X-Axis
  (bind _x_movement_distance (Timeline|PlatformMovement_Timeline%202 PlayFromStart)
    (:Update
      (Transformation|SetActorRelativeLocation (+ _x_movement_distance (Variables|Default|GetInitial%20Platform%20Location))))))

(fn ConstructionScript)