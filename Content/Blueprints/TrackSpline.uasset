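; Spline-driven race track builder that generates road meshes, optional turbo pads and guard rails in its construction script.
; It syncs a per-point RoadDataArray to the spline's point count, padding with defaults or trimming the last entry.
; Each enabled segment gets spline mesh components that blend bank, width and thickness between neighbouring points, with optional loop closure and collision.
; Optional text labels show point indices for editing.
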(fn ConstructionScript
  (Utilities|FlowControl|Sequence
    (:then_0
      (CallFunction|FindNumberOfSplinePoints))
    (:then_1
      (CallFunction|LoadRoadDataArray))
    (:then_2
      (CallFunction|SpawnStaticMesh))
    (:then_3
      (CallFunction|DisplaySplinePointNumber))))

(fn LoadRoadDataArray
  (bind _road_data_array (Variables|TrackSetup|GetRoad%20Data%20Array))
  ;[0 0 0] For every Spline Point, set the Struct to the Road Mesh Default
  (Math|Integer|CompareInt (Utilities|Array|Length (Variables|TrackSetup|GetRoad%20Data%20Array)) (Variables|Loops|GetNumber%20of%20Spline%20Points) :!label _label ; If Road Data Aray Length < Number of Spline Points \n          Add to the Data Array && Loop Function\n\nIf Road Data Array Length > Number of Spline Points\n          Remove the Last Index of the Road Data Array Index
    (:>
      (Utilities|Array|RemoveIndex _road_data_array (Utilities|Array|LastIndex _road_data_array)) ; If the Data Array is longer than the\nNumber of Spline Points\nRemove the Last Index
    )
    (:<
      (Utilities|Array|Add (Variables|TrackSetup|GetRoad%20Data%20Array) (Variables|TrackSetup|GetRoad%20Mesh%20Default)) ; If the Data Array is less than the\nNumber of Spline Points\nAdd an Item to the Array\n\nThen checks again
      (goto _label))))

(fn FindNumberOfSplinePoints
  ;[0 0 0] Gets the number of Spline Points, and adds that number to a Global Variable for reference
  (Variables|Loops|SetNumber%20of%20Spline%20Points (Spline|GetNumberOfSplinePoints (Variables|Default|GetSpline))))

(fn BuildTrackElement
  (params (Loop%20Index :type Integer) (Track%20Element%20Mesh :type Static%20Mesh%20Object%20Reference))
  (LocalVariables|SetLocal_Current%20Loop%20Index Loop%20Index)
  (LocalVariables|SetLocal_Next%20Loop%20Index (Math|Integer|%(Integer) (+ Loop%20Index 1) (Variables|Loops|GetNumber%20of%20Spline%20Points)))
  (LocalVariables|SetLocal_Track%20Element%20Mesh Track%20Element%20Mesh) ; Holds the mech that will be applied \nto each Spline Point
  (Utilities|FlowControl|Sequence
    (:then_0
      ;[0 0 0] Stores Start Location & Tangent, and End Location & Tangent (Current & Next Spline Location)
      (LocalVariables|SetLocal_Start%20Location (.Location (Spline|GetLocationandTangentatSplinePoint (Variables|Default|GetSpline) (LocalVariables|GetLocal_Current%20Loop%20Index) "Local")))
      (LocalVariables|SetLocal_Start%20Tangent (.Tangent (Spline|GetLocationandTangentatSplinePoint (Variables|Default|GetSpline) (LocalVariables|GetLocal_Current%20Loop%20Index) "Local")))
      (LocalVariables|SetLocal_End%20Location (.Location (Spline|GetLocationandTangentatSplinePoint (Variables|Default|GetSpline) (LocalVariables|GetLocal_Next%20Loop%20Index) "Local")))
      (LocalVariables|SetLocal_End%20Tangent (.Tangent (Spline|GetLocationandTangentatSplinePoint (Variables|Default|GetSpline) (LocalVariables|GetLocal_Next%20Loop%20Index) "Local")))
      ;[0 0 0] Gets data for the Start & End of Spline Mesh
      (LocalVariables|SetLocal_Start%20Roll (.trackbank (Utilities|Array|Get(acopy) (Variables|TrackSetup|GetRoad%20Data%20Array) (LocalVariables|GetLocal_Current%20Loop%20Index))))
      (LocalVariables|SetLocal_Start%20Scale (Math|Vector2D|MakeVector2D (.trackwidth (Utilities|Array|Get(acopy) (Variables|TrackSetup|GetRoad%20Data%20Array) (LocalVariables|GetLocal_Current%20Loop%20Index))) (.thickness (Utilities|Array|Get(acopy) (Variables|TrackSetup|GetRoad%20Data%20Array) (LocalVariables|GetLocal_Current%20Loop%20Index)))))
      (LocalVariables|SetLocal_End%20Roll (.trackbank (Utilities|Array|Get(acopy) (Variables|TrackSetup|GetRoad%20Data%20Array) (LocalVariables|GetLocal_Next%20Loop%20Index))))
      (LocalVariables|SetLocal_End%20Scale (Math|Vector2D|MakeVector2D (.trackwidth (Utilities|Array|Get(acopy) (Variables|TrackSetup|GetRoad%20Data%20Array) (LocalVariables|GetLocal_Next%20Loop%20Index))) (.thickness (Utilities|Array|Get(acopy) (Variables|TrackSetup|GetRoad%20Data%20Array) (LocalVariables|GetLocal_Next%20Loop%20Index))))))
    (:then_1
      (bind _returnvalue (AddComponent|AddSplineMeshComponent false))
      (LocalVariables|SetLocal_Current%20Spline%20Mesh _returnvalue) ; Local Variable for keeping Blueprint clean
      (Components|StaticMesh|SetStaticMesh (LocalVariables|GetLocal_Current%20Spline%20Mesh) (LocalVariables|GetLocal_Track%20Element%20Mesh))
      (SplineMesh|SetStartandEnd (LocalVariables|GetLocal_Current%20Spline%20Mesh) (LocalVariables|GetLocal_Start%20Location) (LocalVariables|GetLocal_Start%20Tangent) (LocalVariables|GetLocal_End%20Location) (LocalVariables|GetLocal_End%20Tangent) true :!class /Script/Engine.SplineMeshComponent) ; Lecation between each Spline Point\nwhere the Static Mesh is Spawned
      ;[0 0 0] Sets Start & End Roll for the Spline Mesh
      ; Rotation of each Static Mesh
      (Class|SplineMeshComponent|SetStartRoll (LocalVariables|GetLocal_Current%20Spline%20Mesh) (LocalVariables|GetLocal_Start%20Roll) true)
      (Class|SplineMeshComponent|SetEndRoll (LocalVariables|GetLocal_Current%20Spline%20Mesh) (LocalVariables|GetLocal_End%20Roll) true)
      ;[0 0 0] Sets Start & End of Spline Mesh Scale
      ; Size of each Static Mesh
      (SplineMesh|SetStartScale (LocalVariables|GetLocal_Current%20Spline%20Mesh) (LocalVariables|GetLocal_Start%20Scale) true :!class /Script/Engine.SplineMeshComponent)
      (SplineMesh|SetEndScale (LocalVariables|GetLocal_Current%20Spline%20Mesh) (LocalVariables|GetLocal_End%20Scale) true :!class /Script/Engine.SplineMeshComponent)
      ;[0 0 0] If True: Enable Collision on Spline Mesh
      (Collision|SetCollisionEnabled (LocalVariables|GetLocal_Current%20Spline%20Mesh) (select (Variables|Debugging|GetCollision) "QueryAndPhysics" "NoCollision")))))

(fn DisplaySplinePointNumber
  ;[0 0 0] Generates & Displays Number of the Spline Array Index for each Spline Point
  (if (Variables|Debugging|GetShow%20Spline%20Point%20Numbers) ; Turns text rendering\nOn/Off
    (for _index (range 0 (- (Variables|Loops|GetNumber%20of%20Spline%20Points) 1)) ; For every Spline Point\nDraw Text that shows the Spline Point Number
      (LocalVariables|SetLocal_Spline%20Index _index) ; Local Variable to keep the Blueprint clean
      (bind _returnvalue (AddComponent|AddTextRenderComponent false (Math|Transform|MakeTransform (Math|Vector|MakeVector (.X (Math|Vector|BreakVector (.Location (Spline|GetLocationandTangentatSplinePoint (Variables|Default|GetSpline) (LocalVariables|GetLocal_Spline%20Index) "Local")))) (.Y (Math|Vector|BreakVector (.Location (Spline|GetLocationandTangentatSplinePoint (Variables|Default|GetSpline) (LocalVariables|GetLocal_Spline%20Index) "Local")))) (+ (.Z (Math|Vector|BreakVector (.Location (Spline|GetLocationandTangentatSplinePoint (Variables|Default|GetSpline) (LocalVariables|GetLocal_Spline%20Index) "Local")))) 5e+01)) (Math|Conversions|RotationFromXVector (Math|Vector|MakeVector (.X (Math|Vector|BreakVector (* (.Tangent (Spline|GetLocationandTangentatSplinePoint (Variables|Default|GetSpline) (LocalVariables|GetLocal_Spline%20Index) "Local")) -1.0))) (.Y (Math|Vector|BreakVector (* (.Tangent (Spline|GetLocationandTangentatSplinePoint (Variables|Default|GetSpline) (LocalVariables|GetLocal_Spline%20Index) "Local")) -1.0))) (- (.Z (Math|Vector|BreakVector (* (.Tangent (Spline|GetLocationandTangentatSplinePoint (Variables|Default|GetSpline) (LocalVariables|GetLocal_Spline%20Index) "Local")) -1.0))) 0.0))))))
      (Rendering|Components|TextRender|SetText _returnvalue (Utilities|Text|ToText(Integer) (LocalVariables|GetLocal_Spline%20Index))) ; Prints the Spline Index Number above the Spline Point
    )))

(fn SpawnStaticMesh
  ;[0 0 0] For each Spline Point, place a Spline Mesh between each point
  (for _index (range 0 (- (Variables|Loops|GetNumber%20of%20Spline%20Points) (Math|Integer|SelectInt 1 2 (Variables|TrackSetup|GetLooping%20Track)))) ; Construction Loop\n\nFor each item in the Data Array\nSpawn the Corresponding Static Mesh
    (bind _output_get (LocalVariables|SetLocal_Current%20Loop%20Index _index))
    (if (.spawnmesh (Utilities|Array|Get(acopy) (Variables|TrackSetup|GetRoad%20Data%20Array) _output_get))
      (Utilities|FlowControl|Sequence
        (:then_0
          ;;[0.03299 0.03299 0.03299] Spawns Bottom, Turbo Pads, Left, Right meshes when applicable at Current Loop Index
          (if (.turbopad (Utilities|Array|Get(acopy) (Variables|TrackSetup|GetRoad%20Data%20Array) _output_get)) ; if Ture: Spawn a Turbo Pad Mesh\nIf False: Spawn regular ROad Mesh
            (CallFunction|BuildTrackElement (LocalVariables|GetLocal_Current%20Loop%20Index) (Variables|Meshes|GetRoad%20Mesh_Turbo%20Pad))
            (else
              (CallFunction|BuildTrackElement (LocalVariables|GetLocal_Current%20Loop%20Index) (Variables|Meshes|GetRoad%20Mesh)))))
        (:then_1
          (if (.leftguardrail (Utilities|Array|Get(acopy) (Variables|TrackSetup|GetRoad%20Data%20Array) _output_get)) ; Spawns Left Guard Rail if True
            (CallFunction|BuildTrackElement (LocalVariables|GetLocal_Current%20Loop%20Index) (Variables|Meshes|GetRoad%20Mesh_Left%20Guard%20Rail))))
        (:then_2
          (if (.rightguardrail (Utilities|Array|Get(acopy) (Variables|TrackSetup|GetRoad%20Data%20Array) _output_get)) ; Spawns Right Guard Rail if True
            (CallFunction|BuildTrackElement (LocalVariables|GetLocal_Current%20Loop%20Index) (Variables|Meshes|GetRoad%20Mesh_Right%20Guard%20Rail))))))))