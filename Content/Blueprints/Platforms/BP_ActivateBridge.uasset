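; BP_ActivateBridge is a triggered moving platform that carries the overlapping actor from a start to an end location.
; Trigger overlap starts a delayed timeline that lerps the platform, while Tick pins the actor above it.
; Reaching the EndLocation overlap releases the actor and initializes followers once.
; When the physics ball leaves the trigger, the timeline reverses after a delay; the sound call is unconnected.
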(event OnComponentBeginOverlap(EndLocation)
  (params (OverlappedComponent :type Primitive%20Component%20Object%20Reference) (OtherActor :type Actor%20Object%20Reference) (OtherComp :type Primitive%20Component%20Object%20Reference) (OtherBodyIndex :type Integer) (bFromSweep :type Boolean) (SweepResult :type Hit%20Result%20Structure%20%28by%20ref%29))
  ;[0 0 0] When you reach the EndLocation, detach the Player from the Elevator
  (Variables|Default|SetElevator%20Activated false)
  ;[0 0 0] Sets the Followers to chase the Player
  (Utilities|FlowControl|DoOnce false
    (:Completed
      (Default|CallInitializeFollowers))))

(event OnComponentEndOverlap(Trigger)
  (params (OverlappedComponent :type Primitive%20Component%20Object%20Reference) (OtherActor :type Actor%20Object%20Reference) (OtherComp :type Primitive%20Component%20Object%20Reference) (OtherBodyIndex :type Integer))
  ;[0 0 0] If the Player leaves the Elevator, move the elevator back to the Start Location
  (Utilities|Casting|CastToPhysicsBallBP OtherActor)
  (Utilities|FlowControl|Delay 5.0)
  ;[0 0 0] Moves the platform from the Start Location to the End Location
  (bind _movement_forward (Timeline|ForwardMovement Reverse)
    (:Update
      (Transformation|SetRelativeLocation (Variables|Default|GetActivatedPlatform) (Math|Vector|Lerp(Vector) (Variables|Default|GetStartLoc) (Variables|/Script/Engine.SceneComponent|GetRelativeLocation (Variables|Default|GetEndLocation)) _movement_forward) false false))))

(event OnComponentBeginOverlap(Trigger)
  (params (OverlappedComponent :type Primitive%20Component%20Object%20Reference) (OtherActor :type Actor%20Object%20Reference) (OtherComp :type Primitive%20Component%20Object%20Reference) (OtherBodyIndex :type Integer) (bFromSweep :type Boolean) (SweepResult :type Hit%20Result%20Structure%20%28by%20ref%29))
  ;[0 0 0] Moves the platform from the Start Location to the End Location
  (Variables|Default|SetElevator%20Activated true)
  (Utilities|FlowControl|Delay 0.5)
  (bind _movement_forward (Timeline|ForwardMovement Play)
    (:Update
      (Transformation|SetRelativeLocation (Variables|Default|GetActivatedPlatform) (Math|Vector|Lerp(Vector) (Variables|Default|GetStartLoc) (Variables|/Script/Engine.SceneComponent|GetRelativeLocation (Variables|Default|GetEndLocation)) _movement_forward) false false))))

(event EventTick
  (params (DeltaSeconds :type Float%20%28single-precision%29))
  ;[0 0 0] Keeps Ball on the centre location of the Elevator while it is moving
  (if (Variables|Default|GetElevator%20Activated)
    (Transformation|SetActorRelativeLocation (stale OnComponentBeginOverlap(Trigger) OtherActor) (+ "0, 0,30.000000" (Transformation|GetWorldLocation (Variables|Default|GetActivatedPlatform))))))

(fn ConstructionScript)